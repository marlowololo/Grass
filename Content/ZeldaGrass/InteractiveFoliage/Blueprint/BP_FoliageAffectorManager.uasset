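; Manager actor that feeds the positions and radii of scene foliage affectors to a Niagara grid system for interactive foliage.
; On BeginPlay it caches every AC_SceneFoliageAffector component on actors tagged FoliageAffector.
; Each Tick it packs their location and radius into a Vector4 array and pushes it to the Niagara user parameter.
; An unconnected variant of the same logic using AC_FoliageAffector remains in the graph.
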(event EventBeginPlay
  (bind _outactors (Actor|GetAllActorswithTag "FoliageAffector"))
  (for _array_element _outactors
    (for _array_element_2 (Actor|GetComponentsByClass _array_element "/Game/ZeldaGrass/InteractiveFoliage/Blueprint/AC_SceneFoliageAffector.AC_SceneFoliageAffector_C")
      (Utilities|IsValid _array_element_2
        (:Is%20Valid
          (Utilities|Array|Add (Variables|Default|GetSceneFoliageAffectorList) _array_element_2)
          (Math|Integer|IncrementInt (Variables|Default|GetNumOfAffector))))))
  (Utilities|Array|Resize (Variables|Default|GetLocationAndRadius) (Utilities|Array|Length (Variables|Default|GetSceneFoliageAffectorList))))

(event EventTick
  (params (DeltaSeconds :type Float%20%28single-precision%29))
  (for (_array_element _array_index) (Variables|Default|GetSceneFoliageAffectorList)
    (bind _locationandradius (Default|GetLocationandRadius _array_element))
    (Utilities|Array|SetArrayElem (Variables|Default|GetLocationAndRadius) _array_index _locationandradius))
  (Class|NiagaraDataInterfaceArrayFunctionLibrary|SetNiagaraArrayVector4 (Variables|Default|GetNS_FoliageAffectorGrid) "User.LocationsAndRadius" (Variables|Default|GetLocationAndRadius)))

(fn ConstructionScript)