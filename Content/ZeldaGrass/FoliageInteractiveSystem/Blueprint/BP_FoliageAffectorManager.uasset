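; BP_FoliageAffectorManager feeds the positions and radii of foliage affectors to a Niagara grid system for interactive foliage.
; On BeginPlay it gathers AC_FoliageAffector components from actors tagged "FoliageAffector" and sizes a LocationAndRadius array to the tagged actor count.
; Each Tick it refreshes that array from every component and pushes it to NSFoliageAffectorGrid as a Vector4 array user parameter.
; Affectors are collected only once, at BeginPlay.
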(event EventBeginPlay
  (bind _outactors (Actor|GetAllActorswithTag "FoliageAffector"))
  (Utilities|Array|Resize (Variables|Default|GetLocationAndRadius) (Utilities|Array|Length _outactors))
  (for _array_element _outactors
    (Utilities|IsValid (Actor|GetComponentbyClass _array_element "/Game/ZeldaGrass/FoliageInteractiveSystem/Blueprint/AC_FoliageAffector.AC_FoliageAffector_C")
      (:Is%20Valid
        (Utilities|Array|Add (Variables|Default|GetFoliageAffectorList) (Actor|GetComponentbyClass _array_element "/Game/ZeldaGrass/FoliageInteractiveSystem/Blueprint/AC_FoliageAffector.AC_FoliageAffector_C"))))))

(event EventTick
  (params (DeltaSeconds :type Float%20%28single-precision%29))
  (for (_array_element _array_index) (Variables|Default|GetFoliageAffectorList)
    (bind _locationandradius (Default|GetLocationandRadius _array_element))
    (Utilities|Array|SetArrayElem (Variables|Default|GetLocationAndRadius) _array_index _locationandradius))
  (Class|NiagaraDataInterfaceArrayFunctionLibrary|SetNiagaraArrayVector4 (Variables|Default|GetNS_FoliageAffectorGrid) "User.LocationsAndRadius" (Variables|Default|GetLocationAndRadius)))

(fn ConstructionScript)